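; A wandering NPC character that roams the level and flags when the third-person player character is near it.
; On BeginPlay it picks a random walk speed, then loops AIMoveTo to random reachable points within a radius, pausing randomly after success or failure.
; Its box overlap sets or clears AIOverlap on the player character and prints a debug greeting or farewell.
; TalkEvent is an empty stub.
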(event `self.ReceiveBeginPlay`
  (bind _output_get (set `self.walkspeed` (`KismetMathLibrary.RandomFloatInRange` 100.0 450.0)))
  (set `CharacterMovementComponent.MaxWalkSpeed` _output_get (`self.CharacterMovement`))
  (`self.walkEvent`))

(event `walkEvent`
  (if (not (`self.waiking`))
    (`|AIMoveTo` self (`NavigationSystemV1.K2_GetRandomReachablePointInRadius` (`self.K2_GetActorLocation`) (`self.walkRadius`) null null) null
      (:`then`
        (set `self.waiking` true))
      (:`OnSuccess`
        (`KismetSystemLibrary.Delay` (`KismetMathLibrary.RandomFloatInRange` 1.0 5.0) :!label _label)
        (set `self.waiking` false)
        (`self.walkEvent`))
      (:`OnFail`
        (goto _label)))))

(event `self.Box.OnComponentBeginOverlap`
  (params (OverlappedComponent :type "PrimitiveComponent Object Reference") (OtherActor :type "Actor Object Reference") (OtherComp :type "PrimitiveComponent Object Reference") (OtherBodyIndex :type Integer) (bFromSweep :type Boolean) (SweepResult :type "HitResult Structure (by ref)"))
  (bind _asbp_third_person_character (cast `/Game/ThirdPerson/Blueprints/BP_ThirdPersonCharacter` OtherActor))
  (set `/Game/ThirdPerson/Blueprints/BP_ThirdPersonCharacter.AI_overlap` true _asbp_third_person_character)
  (`KismetSystemLibrary.PrintString` "Hello"))

(event `self.Box.OnComponentEndOverlap`
  (params (OverlappedComponent :type "PrimitiveComponent Object Reference") (OtherActor :type "Actor Object Reference") (OtherComp :type "PrimitiveComponent Object Reference") (OtherBodyIndex :type Integer))
  (bind _asbp_third_person_character (cast `/Game/ThirdPerson/Blueprints/BP_ThirdPersonCharacter` OtherActor))
  (set `/Game/ThirdPerson/Blueprints/BP_ThirdPersonCharacter.AI_overlap` false _asbp_third_person_character)
  (`KismetSystemLibrary.PrintString` "Bye"))

(event `TalkEvent`)

(fn `UserConstructionScript`)